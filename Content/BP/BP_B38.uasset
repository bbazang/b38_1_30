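; BP_B38 is a player-controlled twin-propeller airplane pawn that flies forward continuously.
; Each tick it spins both propellers and moves along local X, both scaled by NewVar and delta time, while also adding forward movement input.
; Pitch and roll axis inputs rotate the actor locally, scaled by Speed and delta time, with no yaw control.
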(event `self.ReceiveTick`
  (params (DeltaSeconds :type "Float (single-precision)"))
  (`SceneComponent.K2_AddLocalRotation` (`self.SM_P38_Propeller`) (`KismetMathLibrary.MakeRotator` (* (`GameplayStatics.GetWorldDeltaSeconds`) (`self.NewVar`))) false false)
  (`SceneComponent.K2_AddLocalRotation` (`self.SM_P38_Propeller1`) (`KismetMathLibrary.MakeRotator` (* (`GameplayStatics.GetWorldDeltaSeconds`) (`self.NewVar`))) false false)
  (`self.AddMovementInput` (`self.GetActorForwardVector`))
  ;[1 1 1] 비행기이동
  (`self.K2_AddActorLocalOffset` (`KismetMathLibrary.MakeVector` (* (`GameplayStatics.GetWorldDeltaSeconds`) (`self.NewVar`)))))

(event `InputAxis|pitch`
  (params (AxisValue :type "Float (single-precision)"))
  ;[1 0.224 0.224] 피치 회전
  (`self.K2_AddActorLocalRotation` (`KismetMathLibrary.MakeRotator` 0.0 (* AxisValue (`GameplayStatics.GetWorldDeltaSeconds`) (`self.speed`)))))

(event `InputAxis|roll`
  (params (AxisValue :type "Float (single-precision)"))
  ;[1 1 1] 롤회전
  (`self.K2_AddActorLocalRotation` (`KismetMathLibrary.MakeRotator` (* AxisValue (`GameplayStatics.GetWorldDeltaSeconds`) (`self.speed`)))))

(fn `UserConstructionScript`)